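; Shots is a projectile actor that damages either a Boss1 or a BP_dragonslayer1 on overlap.
; On BeginPlay it sets its ProjectileMovement velocity to a fixed speed along the X axis.
; Its Capsule overlap checks for Boss1 and its Sphere overlap for BP_dragonslayer1, each destroying the projectile and directly subtracting a fixed amount from that target's health variable.
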(event OnComponentBeginOverlap(Sphere)
  (params (OverlappedComponent :type Primitive%20Component%20Object%20Reference) (OtherActor :type Actor%20Object%20Reference) (OtherComp :type Primitive%20Component%20Object%20Reference) (OtherBodyIndex :type Integer) (bFromSweep :type Boolean) (SweepResult :type Hit%20Result%20Structure%20%28by%20ref%29))
  (bind _asbp_dragonslayer_1 (Utilities|Casting|CastToBP_dragonslayer1 OtherActor))
  (Actor|DestroyActor)
  (Variables|/Game/DreamLife/blueprint/BP_dragonslayer1.BP_dragonslayer1_C|SetHealth_Now _asbp_dragonslayer_1 (- (Variables|/Game/DreamLife/blueprint/BP_dragonslayer1.BP_dragonslayer1_C|GetHealth_Now _asbp_dragonslayer_1) 0.2)))

(event OnComponentBeginOverlap(Capsule)
  (params (OverlappedComponent :type Primitive%20Component%20Object%20Reference) (OtherActor :type Actor%20Object%20Reference) (OtherComp :type Primitive%20Component%20Object%20Reference) (OtherBodyIndex :type Integer) (bFromSweep :type Boolean) (SweepResult :type Hit%20Result%20Structure%20%28by%20ref%29))
  (bind _asboss_1 (Utilities|Casting|CastToBoss1 OtherActor))
  (Actor|DestroyActor)
  (Variables|/Game/DreamLife/blueprint/Boss1.Boss1_C|SetHealth _asboss_1 (- (Variables|/Game/DreamLife/blueprint/Boss1.Boss1_C|GetHealth _asboss_1) 3)))

(event EventBeginPlay
  (Variables|/Script/Engine.MovementComponent|SetVelocity (Variables|Default|GetProjectileMovement) "1000.000000, 0,0.000000"))

(event Input|AxisEvents|InputAxisMoveRight
  (params (AxisValue :type Float%20%28single-precision%29)))

(fn ConstructionScript)