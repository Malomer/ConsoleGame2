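; BP_dragonslayer1 is a 2D flipbook character that walks along X, damages any BP_dragonslayer overlapping its box, and loses health on that contact.
; Tick destroys it at low health, otherwise updates animation, mirrors the sprite by X velocity, and applies movement, using a FlipFlop when stalled to negate direction on alternate passes.
; It also handles Shoot input to spawn Shots at an arrow, and carries an Unpause helper.
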(event OnComponentBeginOverlap(Box)
  (params (OverlappedComponent :type Primitive%20Component%20Object%20Reference) (OtherActor :type Actor%20Object%20Reference) (OtherComp :type Primitive%20Component%20Object%20Reference) (OtherBodyIndex :type Integer) (bFromSweep :type Boolean) (SweepResult :type Hit%20Result%20Structure%20%28by%20ref%29))
  (bind _asbp_dragonslayer (Utilities|Casting|CastToBP_dragonslayer OtherActor))
  (Default|Damage _asbp_dragonslayer (Variables|Default|Getdamagenow))
  (Variables|Default|SetHealth_Now (- (Variables|Default|GetHealth_Now) 0.3))
  (if (>= 0.0 (Variables|Default|GetHealth_Now))
    (Actor|DestroyActor)))

(event Custom|UpdateAnimation
  ;[1 1 1] Handle Animation
  (switch Utilities|FlowControl|Switch|SwitchonChat_state (Variables|Default|Getstate)
    (:NewEnumerator3
      (if (Utilities|Enum|Equal(Enum) (Variables|Default|Getstate) "NewEnumerator5")
        (Sprite|SetFlipbook (Variables|Default|GetSprite) "/Game/DreamLife/sprite/character/A_jump.A_jump" :!label _label)
        (else
          (Sprite|SetFlipbook (Variables|Default|GetSprite) (select (> (Math|Vector|VectorLength (Transformation|GetVelocity)) 0.0) "/Game/DreamLife/sprite/character/Run.Run" "/Game/DreamLife/sprite/character/A_Stance.A_Stance") :!label _label_2))))
    (:NewEnumerator4
      (goto _label_2))
    (:NewEnumerator5
      (goto _label))
    (:NewEnumerator7
      (Sprite|SetFlipbook (Variables|Default|GetSprite)))
    (:NewEnumerator8
      (Sprite|SetFlipbook (Variables|Default|GetSprite)))
    (:NewEnumerator9
      (Sprite|SetFlipbook (Variables|Default|GetSprite)))
    (:NewEnumerator10
      (Sprite|SetFlipbook (Variables|Default|GetSprite)))))

(event EventTick
  (params (DeltaSeconds :type Float%20%28single-precision%29))
  (if (>= 0 (Math|Float|Truncate (Variables|Default|GetHealth_Now)))
    (Actor|DestroyActor)
    (else
      (Utilities|FlowControl|Sequence
        (:then_0
          (CallFunction|UpdateAnimation)
          (Math|Float|CompareFloat (.X (Math|Vector|BreakVector (Variables|/Script/Engine.MovementComponent|GetVelocity (Pawn|GetMovementComponent)))) 0.0
            (:>
              (Transformation|SetWorldScale3D (Variables|Default|GetSprite) "1.000000,1.000000,1.000000" :!label _label))
            (:==
              (if (Variables|Default|GetbisMovingRight)
                (goto _label)
                (else
                  (Transformation|SetWorldScale3D (Variables|Default|GetSprite) "-1.000000,1.000000,1.000000" :!label _label_2))))
            (:<
              (goto _label_2))))
        (:then_1
          (Pawn|Input|AddMovementInput "1.000000, 0, 0" (Variables|Default|Getmovement%20) false)
          (if (< (Math|Vector|VectorLength (Transformation|GetVelocity)) 1.0)
            (Utilities|FlowControl|FlipFlop
              (:A
                (Variables|Default|Setmovement%20 (* (Variables|Default|Getmovement%20) -1.0))
                (Variables|Default|SetbisMovingRight true))
              (:B
                (Variables|Default|Setmovement%20 (* (Variables|Default|Getmovement%20) 1.0))
                (Variables|Default|SetbisMovingRight false)))))))))

(event Input|ActionEvents|InputActionShoot
  (params (Key :type Key%20Structure))
  (:Pressed
    (Game|SpawnActorfromClass "/Game/DreamLife/blueprint/shots.shots_C" (Math|Conversions|ToTransform(Vector) (Transformation|GetWorldLocation (Variables|Default|GetArrow1))) "AdjustIfPossibleButDontSpawnIfColliding" 0 0)
    (CallFunction|UpdateAnimation)
    (Variables|Default|Setstate "NewEnumerator3"))
  (:Released
    (Utilities|FlowControl|RetriggerableDelay 0.2)
    (Variables|Default|Setstate "NewEnumerator3")
    (CallFunction|UpdateAnimation)))

(fn ConstructionScript)

(fn Unpause
  (bind _returnvalue (Game|GetPlayerController 0))
  (Game|SetGamePaused false)
  (Viewport|RemoveAllWidgets)
  (Input|SetInputModeGameOnly _returnvalue)
  (Variables|/Script/Engine.PlayerController|SetbShowMouseCursor _returnvalue false))