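; Paper2D boss that teleports between fixed spots and fires bullet patterns, opening on the Transcendance barrage at BeginPlay.
; Tick uses a latent Delay as attack timer, then picks a non-repeating random pattern: barrage, scaled-up Mega Shot, or two-sided Spray.
; Sequences with staggered delays replay shot volleys; a fourth pattern is an unreachable stub.
; Low Health resets the attack interval; zero clears the flipbook and loads MainMenu.
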(event EventBeginPlay
  ;[1 1 1] Attack Pattern 1 (Trancendance)
  (Transformation|SetActorLocation "0, 0,191.000000" false true)
  (Utilities|FlowControl|Delay 2.0)
  (Utilities|FlowControl|Sequence
    (:then_0
      (Game|SpawnActorfromClass "/Game/DreamLife/blueprint/BossAttacks/Left_Shots/BossShots1.BossShots1_C" (Math|Transform|MakeTransform (Transformation|GetWorldLocation (Variables|Collision|GetCapsuleComponent))) "AdjustIfPossibleButDontSpawnIfColliding" 0 0 :!label _label)
      (Utilities|FlowControl|Delay 0.1)
      (Game|SpawnActorfromClass "/Game/DreamLife/blueprint/BossAttacks/Left_Shots/BossShots2.BossShots2_C" (Math|Transform|MakeTransform (Transformation|GetWorldLocation (Variables|Collision|GetCapsuleComponent))) "AdjustIfPossibleButDontSpawnIfColliding" 0 0)
      (Utilities|FlowControl|Delay 0.1)
      (Game|SpawnActorfromClass "/Game/DreamLife/blueprint/BossAttacks/Left_Shots/BossShots3.BossShots3_C" (Math|Transform|MakeTransform (Transformation|GetWorldLocation (Variables|Collision|GetCapsuleComponent))) "AdjustIfPossibleButDontSpawnIfColliding" 0 0)
      (Utilities|FlowControl|Delay 0.1)
      (Game|SpawnActorfromClass "/Game/DreamLife/blueprint/BossAttacks/Left_Shots/BossShots4.BossShots4_C" (Math|Transform|MakeTransform (Transformation|GetWorldLocation (Variables|Collision|GetCapsuleComponent))) "AdjustIfPossibleButDontSpawnIfColliding" 0 0)
      (Utilities|FlowControl|Delay 0.1)
      (Game|SpawnActorfromClass "/Game/DreamLife/blueprint/BossAttacks/BossShots5.BossShots5_C" (Math|Transform|MakeTransform (Transformation|GetWorldLocation (Variables|Collision|GetCapsuleComponent))) "AdjustIfPossibleButDontSpawnIfColliding" 0 0)
      (Utilities|FlowControl|Delay 0.1)
      (Game|SpawnActorfromClass "/Game/DreamLife/blueprint/BossAttacks/Right_Shots/BossShots6.BossShots6_C" (Math|Transform|MakeTransform (Transformation|GetWorldLocation (Variables|Collision|GetCapsuleComponent))) "AdjustIfPossibleButDontSpawnIfColliding" 0 0)
      (Utilities|FlowControl|Delay 0.1)
      (Game|SpawnActorfromClass "/Game/DreamLife/blueprint/BossAttacks/Right_Shots/BossShots7.BossShots7_C" (Math|Transform|MakeTransform (Transformation|GetWorldLocation (Variables|Collision|GetCapsuleComponent))) "AdjustIfPossibleButDontSpawnIfColliding" 0 0)
      (Utilities|FlowControl|Delay 0.1)
      (Game|SpawnActorfromClass "/Game/DreamLife/blueprint/BossAttacks/Right_Shots/BossShots8.BossShots8_C" (Math|Transform|MakeTransform (Transformation|GetWorldLocation (Variables|Collision|GetCapsuleComponent))) "AdjustIfPossibleButDontSpawnIfColliding" 0 0)
      (Utilities|FlowControl|Delay 0.1)
      (Game|SpawnActorfromClass "/Game/DreamLife/blueprint/BossAttacks/Right_Shots/BossShots9.BossShots9_C" (Math|Transform|MakeTransform (Transformation|GetWorldLocation (Variables|Collision|GetCapsuleComponent))) "AdjustIfPossibleButDontSpawnIfColliding" 0 0))
    (:then_1
      (Utilities|FlowControl|Delay 1.0))
    (:then_2
      (Utilities|FlowControl|Delay 2.0)
      (goto _label))
    (:then_3
      (Utilities|FlowControl|Delay 3.0)
      (goto _label))))

(event Collision|EventActorBeginOverlap
  (params (OtherActor :type Actor%20Object%20Reference)))

(event EventTick
  (params (DeltaSeconds :type Float%20%28single-precision%29))
  (bind _health (Variables|Default|GetHealth))
  (if (<= _health 30)
    (Variables|Default|SetDelay 6))
  (if (>= 0 _health)
    (Utilities|FlowControl|Sequence
      (:then_0
        (Utilities|FlowControl|Delay 1.0)
        (Game|OpenLevel(byName) "MainMenu"))
      (:then_1
        (Sprite|SetFlipbook (Variables|Default|GetSprite))))
    (else
      (Utilities|FlowControl|Delay (Math|Conversions|ToFloat(Integer) (Variables|Default|GetDelay)))
      (bind _output_get (Variables|Default|SetSetPattern (Math|Random|RandomInteger 3) :!label _label))
      (if (== _output_get (Variables|Default|GetCurrentPattern))
        (goto _label)
        (else
          (Variables|Default|SetCurrentPattern (Variables|Default|GetSetPattern))
          (Development|PrintString (Utilities|String|ToString(Integer) (Variables|Default|GetCurrentPattern)))
          (Utilities|FlowControl|Sequence
            (:then_0
              ;[1 1 1] Attack Pattern 1 (Trancendance)
              (if (== 0 (Variables|Default|GetCurrentPattern))
                (Transformation|SetActorLocation "0, 0,191.000000" false true)
                (Utilities|FlowControl|Delay 2.0)
                (Utilities|FlowControl|Sequence
                  (:then_0
                    (Game|SpawnActorfromClass "/Game/DreamLife/blueprint/BossAttacks/Left_Shots/BossShots1.BossShots1_C" (Math|Transform|MakeTransform (Transformation|GetWorldLocation (Variables|Collision|GetCapsuleComponent))) "AdjustIfPossibleButDontSpawnIfColliding" 0 0 :!label _label_2)
                    (Utilities|FlowControl|Delay 0.1)
                    (Game|SpawnActorfromClass "/Game/DreamLife/blueprint/BossAttacks/Left_Shots/BossShots2.BossShots2_C" (Math|Transform|MakeTransform (Transformation|GetWorldLocation (Variables|Collision|GetCapsuleComponent))) "AdjustIfPossibleButDontSpawnIfColliding" 0 0)
                    (Utilities|FlowControl|Delay 0.1)
                    (Game|SpawnActorfromClass "/Game/DreamLife/blueprint/BossAttacks/Left_Shots/BossShots3.BossShots3_C" (Math|Transform|MakeTransform (Transformation|GetWorldLocation (Variables|Collision|GetCapsuleComponent))) "AdjustIfPossibleButDontSpawnIfColliding" 0 0)
                    (Utilities|FlowControl|Delay 0.1)
                    (Game|SpawnActorfromClass "/Game/DreamLife/blueprint/BossAttacks/Left_Shots/BossShots4.BossShots4_C" (Math|Transform|MakeTransform (Transformation|GetWorldLocation (Variables|Collision|GetCapsuleComponent))) "AdjustIfPossibleButDontSpawnIfColliding" 0 0)
                    (Utilities|FlowControl|Delay 0.1)
                    (Game|SpawnActorfromClass "/Game/DreamLife/blueprint/BossAttacks/BossShots5.BossShots5_C" (Math|Transform|MakeTransform (Transformation|GetWorldLocation (Variables|Collision|GetCapsuleComponent))) "AdjustIfPossibleButDontSpawnIfColliding" 0 0)
                    (Utilities|FlowControl|Delay 0.1)
                    (Game|SpawnActorfromClass "/Game/DreamLife/blueprint/BossAttacks/Right_Shots/BossShots6.BossShots6_C" (Math|Transform|MakeTransform (Transformation|GetWorldLocation (Variables|Collision|GetCapsuleComponent))) "AdjustIfPossibleButDontSpawnIfColliding" 0 0)
                    (Utilities|FlowControl|Delay 0.1)
                    (Game|SpawnActorfromClass "/Game/DreamLife/blueprint/BossAttacks/Right_Shots/BossShots7.BossShots7_C" (Math|Transform|MakeTransform (Transformation|GetWorldLocation (Variables|Collision|GetCapsuleComponent))) "AdjustIfPossibleButDontSpawnIfColliding" 0 0)
                    (Utilities|FlowControl|Delay 0.1)
                    (Game|SpawnActorfromClass "/Game/DreamLife/blueprint/BossAttacks/Right_Shots/BossShots8.BossShots8_C" (Math|Transform|MakeTransform (Transformation|GetWorldLocation (Variables|Collision|GetCapsuleComponent))) "AdjustIfPossibleButDontSpawnIfColliding" 0 0)
                    (Utilities|FlowControl|Delay 0.1)
                    (Game|SpawnActorfromClass "/Game/DreamLife/blueprint/BossAttacks/Right_Shots/BossShots9.BossShots9_C" (Math|Transform|MakeTransform (Transformation|GetWorldLocation (Variables|Collision|GetCapsuleComponent))) "AdjustIfPossibleButDontSpawnIfColliding" 0 0))
                  (:then_1
                    (Utilities|FlowControl|Delay 1.0))
                  (:then_2
                    (Utilities|FlowControl|Delay 2.0)
                    (goto _label_2))
                  (:then_3
                    (Utilities|FlowControl|Delay 3.0)
                    (goto _label_2)))))
            (:then_1
              ;[1 1 1] Attack Pattern 2 (Mega Shot)
              (if (== 1 (Variables|Default|GetCurrentPattern))
                (bind _output_get_2 (Variables|Default|SetRandomLocation (Math|Random|RandomInteger 2)))
                (if (== 0 _output_get_2)
                  (Transformation|SetActorLocation "250.000000, 0,5.000000" false true)
                  (Sprite|SetFlipbook (Variables|Default|GetSprite) "/Game/DreamLife/sprite/Enemies/BossPaperL.BossPaperL")
                  (Game|SpawnActorfromClass "/Game/DreamLife/blueprint/BossAttacks/BossShotFollowL.BossShotFollowL_C" (Math|Transform|MakeTransform (Transformation|GetWorldLocation (Variables|Collision|GetCapsuleComponent)) "0, 0, 0" "10.000000,1,10.000000") "AdjustIfPossibleButDontSpawnIfColliding" 0 0)
                  (else
                    (Transformation|SetActorLocation "-250.000000, 0,5.000000" false true)
                    (Sprite|SetFlipbook (Variables|Default|GetSprite) "/Game/DreamLife/sprite/Enemies/BossPaperR.BossPaperR")
                    (Game|SpawnActorfromClass "/Game/DreamLife/blueprint/BossAttacks/BossShotFollowR.BossShotFollowR_C" (Math|Transform|MakeTransform (Transformation|GetWorldLocation (Variables|Collision|GetCapsuleComponent)) "0, 0, 0" "10.000000,1,10.000000") "AdjustIfPossibleButDontSpawnIfColliding" 0 0)))))
            (:then_2
              ;[1 1 1] Attack Pattern 3 (Spray)
              (if (== 2 (Variables|Default|GetCurrentPattern))
                (bind _output_get_3 (Variables|Default|SetRandomLocation (Math|Random|RandomInteger 2)))
                (if (== _output_get_3 0)
                  (Sprite|SetFlipbook (Variables|Default|GetSprite) "/Game/DreamLife/sprite/Enemies/BossPaperL.BossPaperL")
                  (Transformation|SetActorLocation "204.000000, 0,-48.000000" false true)
                  (Utilities|FlowControl|Delay 1.0)
                  (Utilities|FlowControl|Sequence
                    (:then_0
                      (Game|SpawnActorfromClass "/Game/DreamLife/blueprint/BossAttacks/Left_Shots/BossShots4.BossShots4_C" (Math|Transform|MakeTransform (Transformation|GetWorldLocation (Variables|Collision|GetCapsuleComponent))) "AdjustIfPossibleButDontSpawnIfColliding" 0 0 :!label _label_3)
                      (Utilities|FlowControl|Delay 0.1)
                      (Game|SpawnActorfromClass "/Game/DreamLife/blueprint/BossAttacks/Left_Shots/BossShots3.BossShots3_C" (Math|Transform|MakeTransform (Transformation|GetWorldLocation (Variables|Collision|GetCapsuleComponent))) "AdjustIfPossibleButDontSpawnIfColliding" 0 0)
                      (Utilities|FlowControl|Delay 0.1)
                      (Game|SpawnActorfromClass "/Game/DreamLife/blueprint/BossAttacks/Left_Shots/BossShots2.BossShots2_C" (Math|Transform|MakeTransform (Transformation|GetWorldLocation (Variables|Collision|GetCapsuleComponent))) "AdjustIfPossibleButDontSpawnIfColliding" 0 0)
                      (Utilities|FlowControl|Delay 0.1)
                      (Game|SpawnActorfromClass "/Game/DreamLife/blueprint/BossAttacks/Left_Shots/BossShots1.BossShots1_C" (Math|Transform|MakeTransform (Transformation|GetWorldLocation (Variables|Collision|GetCapsuleComponent))) "AdjustIfPossibleButDontSpawnIfColliding" 0 0)
                      (Utilities|FlowControl|Delay 0.1)
                      (Game|SpawnActorfromClass "/Game/DreamLife/blueprint/BossAttacks/Left_Shots/BossShots-2.BossShots-2_C" (Math|Transform|MakeTransform (Transformation|GetWorldLocation (Variables|Collision|GetCapsuleComponent))) "AdjustIfPossibleButDontSpawnIfColliding" 0 0)
                      (Utilities|FlowControl|Delay 0.1)
                      (Game|SpawnActorfromClass "/Game/DreamLife/blueprint/BossAttacks/Left_Shots/BossShots-3.BossShots-3_C" (Math|Transform|MakeTransform (Transformation|GetWorldLocation (Variables|Collision|GetCapsuleComponent))) "AdjustIfPossibleButDontSpawnIfColliding" 0 0)
                      (Utilities|FlowControl|Delay 0.1)
                      (Game|SpawnActorfromClass "/Game/DreamLife/blueprint/BossAttacks/Left_Shots/BossShots-4.BossShots-4_C" (Math|Transform|MakeTransform (Transformation|GetWorldLocation (Variables|Collision|GetCapsuleComponent))) "AdjustIfPossibleButDontSpawnIfColliding" 0 0)
                      (Utilities|FlowControl|Delay 0.2))
                    (:then_1
                      (Utilities|FlowControl|Delay 0.5)
                      (goto _label_3))
                    (:then_2
                      (Utilities|FlowControl|Delay 1.0)
                      (goto _label_3))
                    (:then_3
                      (Utilities|FlowControl|Delay 2.0)
                      (Sprite|SetFlipbook (Variables|Default|GetSprite) "/Game/DreamLife/sprite/Enemies/BossPaperR.BossPaperR")
                      (Transformation|SetActorLocation "-204.000000, 0,-48.000000" false true)
                      (Utilities|FlowControl|Delay 1.0)
                      (Utilities|FlowControl|Sequence
                        (:then_0
                          _)
                        (:then_1
                          (Utilities|FlowControl|Delay 0.5))
                        (:then_2
                          (Utilities|FlowControl|Delay 1.0)))
                      (Game|SpawnActorfromClass "/Game/DreamLife/blueprint/BossAttacks/Right_Shots/BossShots6.BossShots6_C" (Math|Transform|MakeTransform (Transformation|GetWorldLocation (Variables|Collision|GetCapsuleComponent))) "AdjustIfPossibleButDontSpawnIfColliding" 0 0)
                      (Game|SpawnActorfromClass "/Game/DreamLife/blueprint/BossAttacks/Right_Shots/BossShots7.BossShots7_C" (Math|Transform|MakeTransform (Transformation|GetWorldLocation (Variables|Collision|GetCapsuleComponent))) "AdjustIfPossibleButDontSpawnIfColliding" 0 0)
                      (Utilities|FlowControl|Delay 0.1)
                      (Game|SpawnActorfromClass "/Game/DreamLife/blueprint/BossAttacks/Right_Shots/BossShots8.BossShots8_C" (Math|Transform|MakeTransform (Transformation|GetWorldLocation (Variables|Collision|GetCapsuleComponent))) "AdjustIfPossibleButDontSpawnIfColliding" 0 0)
                      (Utilities|FlowControl|Delay 0.1)
                      (Game|SpawnActorfromClass "/Game/DreamLife/blueprint/BossAttacks/Right_Shots/BossShots9.BossShots9_C" (Math|Transform|MakeTransform (Transformation|GetWorldLocation (Variables|Collision|GetCapsuleComponent))) "AdjustIfPossibleButDontSpawnIfColliding" 0 0)
                      (Utilities|FlowControl|Delay 0.1)
                      (Game|SpawnActorfromClass "/Game/DreamLife/blueprint/BossAttacks/Right_Shots/BossShots-8.BossShots-8_C" (Math|Transform|MakeTransform (Transformation|GetWorldLocation (Variables|Collision|GetCapsuleComponent))) "AdjustIfPossibleButDontSpawnIfColliding" 0 0)
                      (Utilities|FlowControl|Delay 0.1)
                      (Game|SpawnActorfromClass "/Game/DreamLife/blueprint/BossAttacks/Right_Shots/BossShots-7.BossShots-7_C" (Math|Transform|MakeTransform (Transformation|GetWorldLocation (Variables|Collision|GetCapsuleComponent))) "AdjustIfPossibleButDontSpawnIfColliding" 0 0)
                      (Utilities|FlowControl|Delay 0.1)
                      (Game|SpawnActorfromClass "/Game/DreamLife/blueprint/BossAttacks/Right_Shots/BossShots-6.BossShots-6_C" (Math|Transform|MakeTransform (Transformation|GetWorldLocation (Variables|Collision|GetCapsuleComponent))) "AdjustIfPossibleButDontSpawnIfColliding" 0 0)
                      (Utilities|FlowControl|Delay 0.1)))
                  (else
                    (Sprite|SetFlipbook (Variables|Default|GetSprite) "/Game/DreamLife/sprite/Enemies/BossPaperR.BossPaperR")
                    (Transformation|SetActorLocation "-204.000000, 0,-48.000000" false true)
                    (Utilities|FlowControl|Delay 1.0)
                    (Utilities|FlowControl|Sequence
                      (:then_0
                        (Game|SpawnActorfromClass "/Game/DreamLife/blueprint/BossAttacks/Right_Shots/BossShots6.BossShots6_C" (Math|Transform|MakeTransform (Transformation|GetWorldLocation (Variables|Collision|GetCapsuleComponent))) "AdjustIfPossibleButDontSpawnIfColliding" 0 0 :!label _label_4)
                        (Utilities|FlowControl|Delay 0.1)
                        (Game|SpawnActorfromClass "/Game/DreamLife/blueprint/BossAttacks/Right_Shots/BossShots7.BossShots7_C" (Math|Transform|MakeTransform (Transformation|GetWorldLocation (Variables|Collision|GetCapsuleComponent))) "AdjustIfPossibleButDontSpawnIfColliding" 0 0)
                        (Utilities|FlowControl|Delay 0.1)
                        (Game|SpawnActorfromClass "/Game/DreamLife/blueprint/BossAttacks/Right_Shots/BossShots8.BossShots8_C" (Math|Transform|MakeTransform (Transformation|GetWorldLocation (Variables|Collision|GetCapsuleComponent))) "AdjustIfPossibleButDontSpawnIfColliding" 0 0)
                        (Utilities|FlowControl|Delay 0.1)
                        (Game|SpawnActorfromClass "/Game/DreamLife/blueprint/BossAttacks/Right_Shots/BossShots9.BossShots9_C" (Math|Transform|MakeTransform (Transformation|GetWorldLocation (Variables|Collision|GetCapsuleComponent))) "AdjustIfPossibleButDontSpawnIfColliding" 0 0)
                        (Utilities|FlowControl|Delay 0.1)
                        (Game|SpawnActorfromClass "/Game/DreamLife/blueprint/BossAttacks/Right_Shots/BossShots-8.BossShots-8_C" (Math|Transform|MakeTransform (Transformation|GetWorldLocation (Variables|Collision|GetCapsuleComponent))) "AdjustIfPossibleButDontSpawnIfColliding" 0 0)
                        (Utilities|FlowControl|Delay 0.1)
                        (Game|SpawnActorfromClass "/Game/DreamLife/blueprint/BossAttacks/Right_Shots/BossShots-7.BossShots-7_C" (Math|Transform|MakeTransform (Transformation|GetWorldLocation (Variables|Collision|GetCapsuleComponent))) "AdjustIfPossibleButDontSpawnIfColliding" 0 0)
                        (Utilities|FlowControl|Delay 0.1)
                        (Game|SpawnActorfromClass "/Game/DreamLife/blueprint/BossAttacks/Right_Shots/BossShots-6.BossShots-6_C" (Math|Transform|MakeTransform (Transformation|GetWorldLocation (Variables|Collision|GetCapsuleComponent))) "AdjustIfPossibleButDontSpawnIfColliding" 0 0)
                        (Utilities|FlowControl|Delay 0.1))
                      (:then_1
                        (Utilities|FlowControl|Delay 0.5)
                        (goto _label_4))
                      (:then_2
                        (Utilities|FlowControl|Delay 1.0)
                        (goto _label_4))
                      (:then_3
                        (Utilities|FlowControl|Delay 2.0)
                        (Sprite|SetFlipbook (Variables|Default|GetSprite) "/Game/DreamLife/sprite/Enemies/BossPaperL.BossPaperL")
                        (Transformation|SetActorLocation "204.000000, 0,-48.000000" false true)
                        (Utilities|FlowControl|Delay 1.0)
                        (Utilities|FlowControl|Sequence
                          (:then_0
                            _)
                          (:then_1
                            (Utilities|FlowControl|Delay 0.5))
                          (:then_2
                            (Utilities|FlowControl|Delay 1.0)))
                        (Game|SpawnActorfromClass "/Game/DreamLife/blueprint/BossAttacks/Left_Shots/BossShots4.BossShots4_C" (Math|Transform|MakeTransform (Transformation|GetWorldLocation (Variables|Collision|GetCapsuleComponent))) "AdjustIfPossibleButDontSpawnIfColliding" 0 0)
                        (Utilities|FlowControl|Delay 0.1)
                        (Game|SpawnActorfromClass "/Game/DreamLife/blueprint/BossAttacks/Left_Shots/BossShots3.BossShots3_C" (Math|Transform|MakeTransform (Transformation|GetWorldLocation (Variables|Collision|GetCapsuleComponent))) "AdjustIfPossibleButDontSpawnIfColliding" 0 0)
                        (Utilities|FlowControl|Delay 0.1)
                        (Game|SpawnActorfromClass "/Game/DreamLife/blueprint/BossAttacks/Left_Shots/BossShots2.BossShots2_C" (Math|Transform|MakeTransform (Transformation|GetWorldLocation (Variables|Collision|GetCapsuleComponent))) "AdjustIfPossibleButDontSpawnIfColliding" 0 0)
                        (Utilities|FlowControl|Delay 0.1)
                        (Game|SpawnActorfromClass "/Game/DreamLife/blueprint/BossAttacks/Left_Shots/BossShots1.BossShots1_C" (Math|Transform|MakeTransform (Transformation|GetWorldLocation (Variables|Collision|GetCapsuleComponent))) "AdjustIfPossibleButDontSpawnIfColliding" 0 0)
                        (Utilities|FlowControl|Delay 0.1)
                        (Game|SpawnActorfromClass "/Game/DreamLife/blueprint/BossAttacks/Left_Shots/BossShots-2.BossShots-2_C" (Math|Transform|MakeTransform (Transformation|GetWorldLocation (Variables|Collision|GetCapsuleComponent))) "AdjustIfPossibleButDontSpawnIfColliding" 0 0)
                        (Utilities|FlowControl|Delay 0.1)
                        (Game|SpawnActorfromClass "/Game/DreamLife/blueprint/BossAttacks/Left_Shots/BossShots-3.BossShots-3_C" (Math|Transform|MakeTransform (Transformation|GetWorldLocation (Variables|Collision|GetCapsuleComponent))) "AdjustIfPossibleButDontSpawnIfColliding" 0 0)
                        (Utilities|FlowControl|Delay 0.1)
                        (Game|SpawnActorfromClass "/Game/DreamLife/blueprint/BossAttacks/Left_Shots/BossShots-4.BossShots-4_C" (Math|Transform|MakeTransform (Transformation|GetWorldLocation (Variables|Collision|GetCapsuleComponent))) "AdjustIfPossibleButDontSpawnIfColliding" 0 0)
                        (Utilities|FlowControl|Delay 0.2)))))))
            (:then_3
              ;[1 1 1] Attack Pattern 4 (?)
              (if (== 3 (Variables|Default|GetCurrentPattern))
                _))))))))

(fn ConstructionScript)