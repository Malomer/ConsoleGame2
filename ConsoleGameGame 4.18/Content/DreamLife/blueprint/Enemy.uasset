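; Paper2D enemy that walks along the X axis and damages the dragonslayer player when its capsule overlaps them.
; Each Tick picks a flipbook from its state and speed, and mirrors the sprite by horizontal velocity.
; When nearly stopped, a FlipFlop alternates the facing flag and negates movement on every other trigger.
; It also carries Pause and Unpause functions for a pause menu widget, not called within this Blueprint.
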(event OnComponentBeginOverlap(CapsuleComponent)
  (params (OverlappedComponent :type Primitive%20Component%20Object%20Reference) (OtherActor :type Actor%20Object%20Reference) (OtherComp :type Primitive%20Component%20Object%20Reference) (OtherBodyIndex :type Integer) (bFromSweep :type Boolean) (SweepResult :type Hit%20Result%20Structure%20%28by%20ref%29))
  (bind _asbp_dragonslayer (Utilities|Casting|CastToBP_dragonslayer OtherActor))
  (Default|Damage _asbp_dragonslayer (Variables|Default|Getdamagenow)))

(event Custom|UpdateAnimation
  ;[1 1 1] Handle Animation
  (switch Utilities|FlowControl|Switch|SwitchonChat_state (Variables|Default|Getstate)
    (:NewEnumerator3
      (if (Utilities|Enum|Equal(Enum) (Variables|Default|Getstate) "NewEnumerator5")
        (Sprite|SetFlipbook (Variables|Default|GetSprite) "/Game/DreamLife/sprite/character/A_jump.A_jump" :!label _label)
        (else
          (Sprite|SetFlipbook (Variables|Default|GetSprite) (select (> (Math|Vector|VectorLength (Transformation|GetVelocity)) 0.0) "/Game/DreamLife/sprite/character/Run.Run" "/Game/DreamLife/sprite/character/A_Stance.A_Stance") :!label _label_2))))
    (:NewEnumerator4
      (goto _label_2))
    (:NewEnumerator5
      (goto _label))
    (:NewEnumerator7
      (Sprite|SetFlipbook (Variables|Default|GetSprite)))
    (:NewEnumerator8
      (Sprite|SetFlipbook (Variables|Default|GetSprite) "/Game/DreamLife/sprite/character/death.death"))
    (:NewEnumerator9
      (Sprite|SetFlipbook (Variables|Default|GetSprite)))
    (:NewEnumerator10
      (Sprite|SetFlipbook (Variables|Default|GetSprite) "/Game/DreamLife/sprite/character/fireing.fireing"))))

(event EventTick
  (params (DeltaSeconds :type Float%20%28single-precision%29))
  (Utilities|FlowControl|Sequence
    (:then_0
      (CallFunction|UpdateAnimation)
      (Math|Float|CompareFloat (.X (Math|Vector|BreakVector (Variables|/Script/Engine.MovementComponent|GetVelocity (Pawn|GetMovementComponent)))) 0.0
        (:>
          (Transformation|SetWorldScale3D (Variables|Default|GetSprite) "1.000000,1.000000,1.000000" :!label _label))
        (:==
          (if (Variables|Default|GetbisMovingRight)
            (goto _label)
            (else
              (Transformation|SetWorldScale3D (Variables|Default|GetSprite) "-1.000000,1.000000,1.000000" :!label _label_2))))
        (:<
          (goto _label_2))))
    (:then_1
      (Pawn|Input|AddMovementInput "1.000000, 0, 0" (Variables|Default|Getmovement) false)
      (if (< (Math|Vector|VectorLength (Transformation|GetVelocity)) 1.0)
        (Utilities|FlowControl|FlipFlop
          (:A
            (Variables|Default|Setmovement (* (Variables|Default|Getmovement) -1.0))
            (Variables|Default|SetbisMovingRight true))
          (:B
            (Variables|Default|Setmovement (* (Variables|Default|Getmovement) 1.0))
            (Variables|Default|SetbisMovingRight false)))))))

(fn ConstructionScript)

(fn Pause
  (Game|SetGamePaused true)
  (Utilities|IsValid (Variables|Default|Getpausemenu)
    (:Is%20Valid
      _)
    (:Is%20Not%20Valid
      (bind _returnvalue (UserInterface|CreateWidget "/Game/DreamLife/blueprint/PauseMenuWidget.PauseMenuWidget_C" (Game|GetPlayerController 0)))
      (Variables|Default|Setpausemenu _returnvalue)))
  (UserInterface|Viewport|AddtoViewport (Variables|Default|Getpausemenu) 0)
  (Input|SetInputModeGameandUI (Game|GetPlayerController 0) (Variables|Default|Getpausemenu) "DoNotLock" true)
  (Variables|/Script/Engine.PlayerController|SetbShowMouseCursor (Game|GetPlayerController 0) true))

(fn Unpause
  (bind _returnvalue (Game|GetPlayerController 0))
  (Game|SetGamePaused false)
  (Viewport|RemoveAllWidgets)
  (Input|SetInputModeGameOnly _returnvalue)
  (Variables|/Script/Engine.PlayerController|SetbShowMouseCursor _returnvalue false))